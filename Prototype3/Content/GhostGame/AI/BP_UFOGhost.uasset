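; UFO ghost enemy character that periodically dashes and moves toward throwable objects.
; Tick-driven Delays pace a dash that launches it at triple its horizontal velocity, then spawns a rear-facing dash VFX when the cooldown ends.
; A second delayed Tick branch sends AIMoveTo at the first actor tagged ThrowableObject, with debug prints.
; Projectile firing logic is present but disconnected, noted as awaiting conversion to a laser.
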(event `self.ReceiveBeginPlay`)

(event `self.ReceiveTick`
  (params (DeltaSeconds :type "Float (single-precision)"))
  (bind (_returnvalue_x _returnvalue_y) (`KismetMathLibrary.BreakVector` (* (`self.GetVelocity`) 3.0)))
  (`parent.ReceiveTick` DeltaSeconds)
  (`|ExecutionSequence`
    (:`then_1`
      ;[1 1 1] Dash
      (`KismetSystemLibrary.Delay` 4.0)
      (if (not (`self.IsDashing`))
        (set `self.IsDashing` true)
        (`self.LaunchCharacter` (`KismetMathLibrary.MakeVector` _returnvalue_x _returnvalue_y))
        (`KismetSystemLibrary.Delay` 5.0)
        (set `self.IsDashing` false)
        (`NiagaraFunctionLibrary.SpawnSystemAtLocation` "/Game/GhostGame/VFX/VFX_GhostDash.VFX_GhostDash" (`self.K2_GetActorLocation`) (`KismetMathLibrary.Conv_VectorToRotator` (* (`KismetMathLibrary.GetForwardVector` (`self.K2_GetActorRotation`)) -1.0)))))
    (:`then_2`
      (`KismetSystemLibrary.Delay` 5.0)
      (bind _outactors (`GameplayStatics.GetAllActorsWithTag` "ThrowableObject"))
      (for _array_element (`|MakeArray` (`|GetArrayItem` _outactors))
        (`|AIMoveTo` self (0.0 0.0 0.0) _array_element 1.0 :!label _label
          (:`then`
            _)
          (:`OnSuccess`
            _))
        (`KismetSystemLibrary.PrintString` "moveto object")
        (`KismetSystemLibrary.Delay` 5.0))
      (goto _label))))

(fn `UserConstructionScript`
  (`parent.UserConstructionScript`))