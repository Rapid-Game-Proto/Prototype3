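; UFO ghost boss that hurls haybales at the player, with an achievement and a return to level select before cull.
; BeginPlay sets health and starts a loop: find the nearest BP_Haybale, glide above it via Timeline, pull it to ProjectileSpawn and fire it.
; Tick uses Delays to pace velocity-based dashes, UFO light spawns and ectoplasm drops.
; Parent BeginPlay and a ballistic-arc projectile solver are left unconnected.
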(event `AttackEvent Hayble`
  ;[1 1 1] Move to Haybale
)

(event `self.AdditionalLogicBeforeCull`
  (bind _asbp_gamemode (cast `/Game/GhostGame/Blueprints/BP_Gamemode` (`GameplayStatics.GetGameMode`)))
  (`/Game/GhostGame/Blueprints/BP_Gamemode.ShowAchievement` _asbp_gamemode 2)
  (bind _asbp_gamemode_2 (cast `/Game/GhostGame/Blueprints/BP_Gamemode` (`GameplayStatics.GetGameMode`)))
  (`/Game/GhostGame/Blueprints/BP_Gamemode.GoToLevelSelect` _asbp_gamemode_2))

(event `self.ReceiveTick`
  (params (DeltaSeconds :type "Float (single-precision)"))
  (bind (_returnvalue_location _returnvalue_rotation) (`KismetMathLibrary.BreakTransform` (`SceneComponent.K2_GetComponentToWorld` (`self.ProjectileSpawn`))))
  (bind (_returnvalue_x _returnvalue_y) (`KismetMathLibrary.BreakVector` (* (`self.GetVelocity`) 5.0)))
  (`parent.ReceiveTick` DeltaSeconds)
  (`|ExecutionSequence`
    (:`then_0`
      ;[1 1 1] Dash
      (`KismetSystemLibrary.Delay` 4.0)
      (if (not (`self.IsDashing`))
        (set `self.IsDashing` true)
        (`self.LaunchCharacter` (`KismetMathLibrary.MakeVector` _returnvalue_x _returnvalue_y))
        (`KismetSystemLibrary.Delay` 5.0)
        (set `self.IsDashing` false)
        (`NiagaraFunctionLibrary.SpawnSystemAtLocation` "/Game/GhostGame/VFX/VFX_GhostDash.VFX_GhostDash" (`self.K2_GetActorLocation`) (`KismetMathLibrary.Conv_VectorToRotator` (* (`KismetMathLibrary.GetForwardVector` (`self.K2_GetActorRotation`)) -1.0)))))
    (:`then_1`
      ;[1 1 1] Spawn UFOlights
      (`KismetSystemLibrary.Delay` 7.5)
      (`AIBlueprintHelperLibrary.SpawnAIFromClass` "/Game/GhostGame/AI/BarnProj/BP_UFOLights.BP_UFOLights_C" null _returnvalue_location _returnvalue_rotation false null)
      (`NiagaraFunctionLibrary.SpawnSystemAtLocation` "/Game/GhostGame/VFX/GhostAppear_VFX_2.GhostAppear_VFX_2" _returnvalue_location (struct) (3.0 3.0 3.0))
      (`NiagaraFunctionLibrary.SpawnSystemAtLocation` "/Game/GhostGame/VFX/GhostAppear_VFX_1.GhostAppear_VFX_1" _returnvalue_location (struct) (3.0 3.0 3.0)))
    (:`then_2`
      ;[1 1 1] Poops Ectoplasm
      (`KismetSystemLibrary.Delay` 4.0)
      (`KismetSystemLibrary.PrintString` "trap droped")
      (if (`self.CanAttack`)
        (`|SpawnActorFromClass` "/Game/GhostGame/AI/BarnProj/BP_Ectoplasm.BP_Ectoplasm_C" (`SceneComponent.K2_GetComponentToWorld` (`self.ProjectileSpawn`)) "AdjustIfPossibleButAlwaysSpawn" "MultiplyWithRoot" null null)))))

(event `self.ReceiveBeginPlay`
  (bind (_endlocation_x _endlocation_y) (`KismetMathLibrary.BreakVector` (`self.EndLocation`)))
  (bind (_returnvalue_x _returnvalue_y) (`KismetMathLibrary.BreakVector` (`self.K2_GetActorLocation` (`self.ClosestProjectile`))))
  (bind (_returnvalue_x_2 _returnvalue_y_2 _returnvalue_z) (`KismetMathLibrary.BreakVector` (`self.K2_GetActorLocation` self)))
  (`|ExecutionSequence`
    (:`then_0`
      (if (`self.CanAttack`) :!label _label
        (bind _outactors (`GameplayStatics.GetAllActorsOfClass` "/Game/GhostGame/AI/BarnProj/BP_Haybale.BP_Haybale_C"))
        (bind _output (`|GetArrayItem` _outactors))
        (set `self.DistancetoProjectile` (`self.GetDistanceTo` _output))
        (set `self.ClosestProjectile` _output)
        (for _array_element _outactors
          (bind _returnvalue (`self.GetDistanceTo` _array_element))
          (if (< _returnvalue (`self.DistancetoProjectile`))
            (set `self.DistancetoProjectile` _returnvalue)
            (set `self.ClosestProjectile` _array_element)))
        (set `self.StartLocation` (`KismetMathLibrary.MakeVector` _returnvalue_x_2 _returnvalue_y_2 _returnvalue_z))
        (set `self.EndLocation` (`KismetMathLibrary.MakeVector` _returnvalue_x _returnvalue_y _returnvalue_z))
        (bind (_direction _movetotimeline) (`Timeline|Timeline` :!via `PlayFromStart`)
          (:`Update`
            (bind _output_get (set `self.EndLocation` (`KismetMathLibrary.MakeVector` _endlocation_x _endlocation_y _returnvalue_z)))
            (`self.K2_SetActorLocation` (`KismetMathLibrary.VLerp` (`self.StartLocation`) _output_get _movetotimeline))
            (`self.Look at Location` (`self.EndLocation`)))
          (:`Finished`
            (`KismetSystemLibrary.PrintString` "Succes")
            (`self.Shot Projectile` (`self.ClosestProjectile`))
            (`KismetSystemLibrary.PrintString` "FIREsucces")
            (`self.AttackEvent Hayble`)
            (goto _label)))))
    (:`then_1`
      (bind _output_get_2 (set `self.MaxHealth` 25.0))
      (set `self.Health` _output_get_2)
      (`self.UpdateHealthBar`))))

(event `self.Box.OnComponentBeginOverlap`
  (params (OverlappedComponent :type "PrimitiveComponent Object Reference") (OtherActor :type "Actor Object Reference") (OtherComp :type "PrimitiveComponent Object Reference") (OtherBodyIndex :type Integer) (bFromSweep :type Boolean) (SweepResult :type "HitResult Structure (by ref)"))
  (cast `/Game/GhostGame/AI/BarnProj/BP_Haybale` OtherActor)
  (`KismetSystemLibrary.PrintString` "Hello")
  (`KismetSystemLibrary.K2_SetTimer` null "Shot Projectile" 0.5 false 0.0 3.0)
  (`KismetSystemLibrary.PrintString` "FIRE"))

(fn `Look at Location`
  (params (`Target Location` :type "Vector Structure"))
  (`self.K2_SetActorRotation` (`KismetMathLibrary.FindLookAtRotation` (`self.K2_GetActorLocation`) `Target Location`)))

(fn `Shot Projectile`
  (params (proj :type "Actor Object Reference"))
  (bind _asbp_haybale (cast `/Game/GhostGame/AI/BarnProj/BP_Haybale` proj))
  (`self.K2_SetActorLocation` _asbp_haybale (`SceneComponent.K2_GetComponentLocation` (`self.ProjectileSpawn`)) false false)
  (`/Game/GhostGame/AI/BP_ProjectilePlaceholder.FireTowardPlayer` _asbp_haybale))

(fn `UserConstructionScript`
  (`parent.UserConstructionScript`))