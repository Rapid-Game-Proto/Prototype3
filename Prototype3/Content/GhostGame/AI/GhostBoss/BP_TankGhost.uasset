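; Tank ghost boss enemy that sets its own boosted health, then awards an achievement and returns to level select before it is culled.
; A looping timer lobs burger projectiles at the player, solving the ballistic equation for the lower launch angle.
; Tick uses parallel Delay chains as cooldowns for velocity-based dashes, burger baby spawns and homing projectiles.
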(event `self.AdditionalLogicBeforeCull`
  (bind _asbp_gamemode (cast `/Game/GhostGame/Blueprints/BP_Gamemode` (`GameplayStatics.GetGameMode`)))
  (`/Game/GhostGame/Blueprints/BP_Gamemode.ShowAchievement` _asbp_gamemode 0)
  (bind _asbp_gamemode_2 (cast `/Game/GhostGame/Blueprints/BP_Gamemode` (`GameplayStatics.GetGameMode`)))
  (`/Game/GhostGame/Blueprints/BP_Gamemode.GoToLevelSelect` _asbp_gamemode_2))

(event `self.ReceiveBeginPlay`
  (`parent.ReceiveBeginPlay`)
  (set `self.Health` (* (`self.Health`) 2.0))
  (`KismetSystemLibrary.K2_SetTimer` null "Shot Projectile" 1.5 true 2.0 3.0)
  (bind _output_get (set `self.MaxHealth` 17.0))
  (set `self.Health` _output_get)
  (`self.UpdateHealthBar`))

(event `self.ReceiveTick`
  (params (DeltaSeconds :type "Float (single-precision)"))
  (bind (_returnvalue_location _returnvalue_rotation) (`KismetMathLibrary.BreakTransform` (`SceneComponent.K2_GetComponentToWorld` (`self.Projectile Spawn`))))
  (bind (_returnvalue_location_2 _returnvalue_rotation_2) (`KismetMathLibrary.BreakTransform` (`SceneComponent.K2_GetComponentToWorld` (`self.Projectile Spawn`))))
  (bind (_returnvalue_x _returnvalue_y) (`KismetMathLibrary.BreakVector` (* (`self.GetVelocity`) 2.0)))
  (`parent.ReceiveTick` DeltaSeconds)
  (`|ExecutionSequence`
    (:`then_0`
      ;[1 1 1] Dash
      (`KismetSystemLibrary.Delay` 5.0)
      (if (not (`self.IsDashing`))
        (set `self.IsDashing` true)
        (`self.LaunchCharacter` (`KismetMathLibrary.MakeVector` _returnvalue_x _returnvalue_y))
        (`KismetSystemLibrary.Delay` 5.0)
        (set `self.IsDashing` false)
        (`NiagaraFunctionLibrary.SpawnSystemAtLocation` "/Game/GhostGame/VFX/VFX_GhostDash.VFX_GhostDash" (`self.K2_GetActorLocation`) (`KismetMathLibrary.Conv_VectorToRotator` (* (`KismetMathLibrary.GetForwardVector` (`self.K2_GetActorRotation`)) -1.0)))))
    (:`then_1`
      ;[1 1 1] Spawn Babies
      (`KismetSystemLibrary.Delay` 8.5)
      (`AIBlueprintHelperLibrary.SpawnAIFromClass` "/Game/GhostGame/AI/DinnerProj/BP_BurgerBabies.BP_BurgerBabies_C" null _returnvalue_location _returnvalue_rotation false null)
      (`NiagaraFunctionLibrary.SpawnSystemAtLocation` "/Game/GhostGame/VFX/GhostAppear_VFX_2.GhostAppear_VFX_2" _returnvalue_location (struct) (3.0 3.0 3.0))
      (`NiagaraFunctionLibrary.SpawnSystemAtLocation` "/Game/GhostGame/VFX/GhostAppear_VFX_1.GhostAppear_VFX_1" _returnvalue_location (struct) (3.0 3.0 3.0)))
    (:`then_2`
      ;[1 1 1] Homing Projectile
      (`KismetSystemLibrary.Delay` 5.0)
      (`|SpawnActorFromClass` "/Game/GhostGame/AI/DinnerProj/BP_Homing_Projectile.BP_Homing_Projectile_C" (`KismetMathLibrary.MakeTransform` _returnvalue_location_2 _returnvalue_rotation_2) "Undefined" "MultiplyWithRoot" null null)
      (`KismetSystemLibrary.PrintText` "fire projectile2"))))

(event `Projectile`
  (`self.Shot Projectile`))

(fn `Shot Projectile`
  (bind (_returnvalue_x _returnvalue_y _returnvalue_z) (`KismetMathLibrary.BreakVector` (`self.K2_GetActorLocation`)))
  (bind _returnvalue (`self.K2_GetActorLocation`))
  (bind _gravity (`self.Gravity`))
  (bind _returnvalue_2 (`KismetMathLibrary.Square` (`self.Velocity`)))
  (bind _outactors (`GameplayStatics.GetAllActorsOfClass` "/Game/GhostGame/Blueprints/BP_Character.BP_Character_C"))
  (for _array_element _outactors
    _)
  (bind (_returnvalue_x_2 _returnvalue_y_2 _returnvalue_z_2) (`KismetMathLibrary.BreakVector` (`self.K2_GetActorLocation` _array_element)))
  (bind _returnvalue_3 (`KismetMathLibrary.VSize2D` (`KismetMathLibrary.MakeVector2D` (- _returnvalue_x_2 _returnvalue_x) (- _returnvalue_y_2 _returnvalue_y))))
  (bind _returnvalue_4 (- (`KismetMathLibrary.Square` _returnvalue_2) (* (+ (* (`KismetMathLibrary.Square` _returnvalue_3) _gravity) (* (* (- _returnvalue_z_2 _returnvalue_z) _returnvalue_2) 2.0)) _gravity)))
  (if (>= _returnvalue_4 0.0)
    (bind (_returnvalue_roll _returnvalue_pitch _returnvalue_yaw) (`KismetMathLibrary.BreakRotator` (`KismetMathLibrary.FindLookAtRotation` _returnvalue (`self.K2_GetActorLocation` _array_element))))
    (bind _returnvalue_5 (`KismetMathLibrary.Sqrt` _returnvalue_4))
    (bind _returnvalue_6 (* _returnvalue_3 _gravity))
    (`|SpawnActorFromClass` "/Game/GhostGame/AI/DinnerProj/BP_BurgerBoss_Projectile.BP_BurgerBoss_Projectile_C" (`KismetMathLibrary.MakeTransform` _returnvalue (`KismetMathLibrary.MakeRotator` _returnvalue_roll (`KismetMathLibrary.FMin` (`KismetMathLibrary.DegAtan` (/ (+ _returnvalue_5 _returnvalue_2) _returnvalue_6)) (`KismetMathLibrary.DegAtan` (/ (- _returnvalue_2 _returnvalue_5) _returnvalue_6))) _returnvalue_yaw)) "Undefined" "MultiplyWithRoot" null null)
    (else
      (`KismetSystemLibrary.PrintString` "unreachable" true true (struct :`R` 1.0 :`G` 0.019406 :`A` 1.0)))))

(fn `UserConstructionScript`
  (`parent.UserConstructionScript`))