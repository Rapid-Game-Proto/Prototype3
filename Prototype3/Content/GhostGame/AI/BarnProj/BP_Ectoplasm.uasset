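; BP_Ectoplasm is a ghost-game hazard that damages the player character while they stand in it.
; Three sphere triggers set a CanAttack flag when a BP_Character enters and clear it on any exit, even if another sphere is still overlapped.
; While the flag is set, Tick calls Attack every frame, applying a small fixed TakeDamage to the BP_Character found by GetActorOfClass, unscaled by delta time.
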(event `self.ReceiveBeginPlay`
  (set `self.CanAttack` false))

(event `self.ReceiveTick`
  (params (DeltaSeconds :type "Float (single-precision)"))
  (if (`self.CanAttack`)
    (`self.Attack`)))

(event `self.Sphere1.OnComponentBeginOverlap`
  (params (OverlappedComponent :type "PrimitiveComponent Object Reference") (OtherActor :type "Actor Object Reference") (OtherComp :type "PrimitiveComponent Object Reference") (OtherBodyIndex :type Integer) (bFromSweep :type Boolean) (SweepResult :type "HitResult Structure (by ref)"))
  (cast `/Game/GhostGame/Blueprints/BP_Character` OtherActor)
  (`KismetSystemLibrary.PrintString` "stepped in ectoplasm1")
  (set `self.CanAttack` true))

(event `self.Sphere2.OnComponentBeginOverlap`
  (params (OverlappedComponent :type "PrimitiveComponent Object Reference") (OtherActor :type "Actor Object Reference") (OtherComp :type "PrimitiveComponent Object Reference") (OtherBodyIndex :type Integer) (bFromSweep :type Boolean) (SweepResult :type "HitResult Structure (by ref)"))
  (cast `/Game/GhostGame/Blueprints/BP_Character` OtherActor)
  (`KismetSystemLibrary.PrintString` "stepped in ectoplasm2")
  (set `self.CanAttack` true))

(event `self.Sphere3.OnComponentBeginOverlap`
  (params (OverlappedComponent :type "PrimitiveComponent Object Reference") (OtherActor :type "Actor Object Reference") (OtherComp :type "PrimitiveComponent Object Reference") (OtherBodyIndex :type Integer) (bFromSweep :type Boolean) (SweepResult :type "HitResult Structure (by ref)"))
  (cast `/Game/GhostGame/Blueprints/BP_Character` OtherActor)
  (`KismetSystemLibrary.PrintString` "stepped in ectoplasm3")
  (set `self.CanAttack` true))

(event `self.Sphere1.OnComponentEndOverlap`
  (params (OverlappedComponent :type "PrimitiveComponent Object Reference") (OtherActor :type "Actor Object Reference") (OtherComp :type "PrimitiveComponent Object Reference") (OtherBodyIndex :type Integer))
  (cast `/Game/GhostGame/Blueprints/BP_Character` OtherActor)
  (set `self.CanAttack` false))

(event `self.Sphere2.OnComponentEndOverlap`
  (params (OverlappedComponent :type "PrimitiveComponent Object Reference") (OtherActor :type "Actor Object Reference") (OtherComp :type "PrimitiveComponent Object Reference") (OtherBodyIndex :type Integer))
  (cast `/Game/GhostGame/Blueprints/BP_Character` OtherActor)
  (set `self.CanAttack` false))

(event `self.Sphere3.OnComponentEndOverlap`
  (params (OverlappedComponent :type "PrimitiveComponent Object Reference") (OtherActor :type "Actor Object Reference") (OtherComp :type "PrimitiveComponent Object Reference") (OtherBodyIndex :type Integer))
  (cast `/Game/GhostGame/Blueprints/BP_Character` OtherActor)
  (set `self.CanAttack` false))

(fn `Attack`
  (bind _returnvalue (`GameplayStatics.GetActorOfClass` "/Game/GhostGame/Blueprints/BP_Character.BP_Character_C"))
  (`/Game/GhostGame/Blueprints/BP_Character.Take Damage` _returnvalue 0.1))

(fn `UserConstructionScript`)