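; UFO light hazard that damages BP_Character while it stands in the beam.
; Begin and end overlaps on both Cone and HitCollider set one shared CanAttack flag, so leaving either clears it.
; While set, Tick calls Attack, which deals fixed per-frame damage, independent of delta time, to the character found by GetActorOfClass.
; Tick also pulses the cone's X and Y scale with a sine wave above its starting size.
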(event `self.ReceiveBeginPlay`
  (`parent.ReceiveBeginPlay`)
  (set `self.CanAttack` false)
  (set `self.OriginScale` (`SceneComponent.K2_GetComponentScale` (`self.Cone`))))

(event `self.ReceiveTick`
  (params (DeltaSeconds :type "Float (single-precision)"))
  (bind (_originscale_x _originscale_y _originscale_z) (`KismetMathLibrary.BreakVector` (`self.OriginScale`)))
  (`parent.ReceiveTick` DeltaSeconds)
  (`|ExecutionSequence`
    (:`then_0`
      (if (`self.CanAttack`)
        (`self.Attack`)))
    (:`then_1`
      (bind _output_get (set `self.Time` (+ DeltaSeconds (`self.Time`))))
      (set `self.Oscillation` (+ (/ (`KismetMathLibrary.Sin` (* _output_get (`self.OscilSpeed`))) 2.0) 0.5))
      (`SceneComponent.SetWorldScale3D` (`self.Cone`) (`KismetMathLibrary.MakeVector` (+ _originscale_x (* (`self.Oscillation`) (`self.OscilMax`))) (+ _originscale_y (* (`self.Oscillation`) (`self.OscilMax`))) _originscale_z)))))

(event `self.HitCollider.OnComponentBeginOverlap`
  (params (OverlappedComponent :type "PrimitiveComponent Object Reference") (OtherActor :type "Actor Object Reference") (OtherComp :type "PrimitiveComponent Object Reference") (OtherBodyIndex :type Integer) (bFromSweep :type Boolean) (SweepResult :type "HitResult Structure (by ref)"))
  (cast `/Game/GhostGame/Blueprints/BP_Character` OtherActor)
  (set `self.CanAttack` true))

(event `self.HitCollider.OnComponentEndOverlap`
  (params (OverlappedComponent :type "PrimitiveComponent Object Reference") (OtherActor :type "Actor Object Reference") (OtherComp :type "PrimitiveComponent Object Reference") (OtherBodyIndex :type Integer))
  (cast `/Game/GhostGame/Blueprints/BP_Character` OtherActor)
  (set `self.CanAttack` false))

(event `self.Cone.OnComponentBeginOverlap`
  (params (OverlappedComponent :type "PrimitiveComponent Object Reference") (OtherActor :type "Actor Object Reference") (OtherComp :type "PrimitiveComponent Object Reference") (OtherBodyIndex :type Integer) (bFromSweep :type Boolean) (SweepResult :type "HitResult Structure (by ref)"))
  ;[1 1 1] Light Damage
  (cast `/Game/GhostGame/Blueprints/BP_Character` OtherActor)
  (set `self.CanAttack` true))

(event `self.Cone.OnComponentEndOverlap`
  (params (OverlappedComponent :type "PrimitiveComponent Object Reference") (OtherActor :type "Actor Object Reference") (OtherComp :type "PrimitiveComponent Object Reference") (OtherBodyIndex :type Integer))
  ;[1 1 1] Light Damage
  (cast `/Game/GhostGame/Blueprints/BP_Character` OtherActor)
  (set `self.CanAttack` false))

(fn `Attack`
  (bind _returnvalue (`GameplayStatics.GetActorOfClass` "/Game/GhostGame/Blueprints/BP_Character.BP_Character_C"))
  (`/Game/GhostGame/Blueprints/BP_Character.Take Damage` _returnvalue 0.18))

(fn `UserConstructionScript`
  (`parent.UserConstructionScript`))