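; Barn boss projectile that aims a ballistic shot at BP_Character and damages it on hit.
; BeginPlay adds all characters to a trace ignore list, then solves the launch-angle equation from Velocity and Gravity, rotating to the flatter arc or printing "unreachable".
; On any Sphere hit it spawns an emitter, traces down to the floor, spawns a BP_ProjectileBarnBoss just above it and destroys itself.
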(event `self.Sphere.OnComponentHit`
  (params (HitComponent :type "PrimitiveComponent Object Reference") (OtherActor :type "Actor Object Reference") (OtherComp :type "PrimitiveComponent Object Reference") (NormalImpulse :type "Vector Structure") (Hit :type "HitResult Structure (by ref)"))
  ;[1 1 1] Deal Damage + Delete in Hit
  (`KismetSystemLibrary.PrintString` (`KismetSystemLibrary.GetDisplayName` OtherActor))
  (bind _asbp_character (cast `/Game/GhostGame/Blueprints/BP_Character` OtherActor)
    (:`then`
      (`/Game/GhostGame/Blueprints/BP_Character.Take Damage` _asbp_character 0.25))
    (:`CastFailed`
      _))
  (`GameplayStatics.SpawnEmitterAttached` null)
  (bind _floorlocation (`self.GetFloorLocationAtPoint` (`self.K2_GetActorLocation`)))
  (`|SpawnActorFromClass` "/Game/GhostGame/AI/BarnProj/BP_ProjectileBarnBoss.BP_ProjectileBarnBoss_C" (`KismetMathLibrary.MakeTransform` (+ _floorlocation (0.0 0.0 40.0)) (`self.K2_GetActorRotation`)) "Undefined" "MultiplyWithRoot" null null)
  (`self.K2_DestroyActor`))

(event `self.Sphere1.OnComponentHit`
  (params (HitComponent :type "PrimitiveComponent Object Reference") (OtherActor :type "Actor Object Reference") (OtherComp :type "PrimitiveComponent Object Reference") (NormalImpulse :type "Vector Structure") (Hit :type "HitResult Structure (by ref)")))

(event `self.ReceiveBeginPlay`
  (bind (_returnvalue_x _returnvalue_y _returnvalue_z) (`KismetMathLibrary.BreakVector` (`self.K2_GetActorLocation`)))
  (bind _returnvalue (`self.K2_GetActorLocation`))
  (bind _gravity (`self.Gravity`))
  (bind _returnvalue_2 (`KismetMathLibrary.Square` (`self.Velocity`)))
  (bind _outactors (`GameplayStatics.GetAllActorsOfClass` "/Game/GhostGame/Blueprints/BP_Character.BP_Character_C"))
  (for _array_element _outactors
    (`KismetArrayLibrary.Array_Set` (`self.IgnoreArray`) 0 _array_element))
  (bind (_returnvalue_x_2 _returnvalue_y_2 _returnvalue_z_2) (`KismetMathLibrary.BreakVector` (`self.K2_GetActorLocation` _array_element)))
  (bind _returnvalue_3 (`KismetMathLibrary.VSize2D` (`KismetMathLibrary.MakeVector2D` (- _returnvalue_x_2 _returnvalue_x) (- _returnvalue_y_2 _returnvalue_y))))
  (bind _returnvalue_4 (- (`KismetMathLibrary.Square` _returnvalue_2) (* (+ (* (`KismetMathLibrary.Square` _returnvalue_3) _gravity) (* (* (- _returnvalue_z_2 _returnvalue_z) _returnvalue_2) 2.0)) _gravity)))
  (if (>= _returnvalue_4 0.0)
    ;[1 1 1] maths :(
    (`self.K2_SetActorLocation` _returnvalue true)
    (bind (_returnvalue_roll _returnvalue_pitch _returnvalue_yaw) (`KismetMathLibrary.BreakRotator` (`KismetMathLibrary.FindLookAtRotation` _returnvalue (`self.K2_GetActorLocation` _array_element))))
    (bind _returnvalue_5 (`KismetMathLibrary.Sqrt` _returnvalue_4))
    (bind _returnvalue_6 (* _returnvalue_3 _gravity))
    (`self.K2_SetActorRotation` (`KismetMathLibrary.MakeRotator` _returnvalue_roll (`KismetMathLibrary.FMin` (`KismetMathLibrary.DegAtan` (/ (+ _returnvalue_5 _returnvalue_2) _returnvalue_6)) (`KismetMathLibrary.DegAtan` (/ (- _returnvalue_2 _returnvalue_5) _returnvalue_6))) _returnvalue_yaw))
    (else
      (`KismetSystemLibrary.PrintString` "unreachable" true true (struct :`R` 1.0 :`G` 0.019406 :`A` 1.0)))))

(fn `GetFloorLocationAtPoint`
  (params (PointLocation :type "Vector Structure"))
  (returns (FloorLocation :type "Vector Structure") (`Success?` :type Boolean))
  (locals (Origin :type "Vector Structure"))
  (bind (_origin_x _origin_y) (`KismetMathLibrary.BreakVector` (`local.Origin`)))
  (set `local.Origin` PointLocation)
  (bind _outhit (`KismetSystemLibrary.LineTraceSingle` PointLocation (- PointLocation (0.0 0.0 99999.0)) "TraceTypeQuery1" true (`self.IgnoreArray`) "None" true (struct :`R` 1.0 :`A` 1.0) (struct :`G` 1.0 :`A` 1.0) 1.0))
  (return (`KismetMathLibrary.MakeVector` _origin_x _origin_y (.z (`.Location` (`GameplayStatics.BreakHitResult` _outhit)))) true))

(fn `UserConstructionScript`)