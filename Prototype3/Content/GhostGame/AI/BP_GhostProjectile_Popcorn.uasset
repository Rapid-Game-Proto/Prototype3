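; BP_GhostProjectile_Popcorn is a ghost projectile variant that homes only briefly after it spawns.
; On BeginPlay it calls LockOnTarget, then switches off homing on its ProjectileMovement after a short delay and destroys itself a few seconds after spawning.
; The parent BeginPlay call is disabled, so this timed sequence replaces any parent startup logic.
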(event `self.ReceiveBeginPlay`
  (`self.LockOnTarget`)
  (`KismetSystemLibrary.Delay` 0.4)
  (set `ProjectileMovementComponent.bIsHomingProjectile` false (`self.ProjectileMovement`))
  (`KismetSystemLibrary.Delay` 2.6)
  (`self.K2_DestroyActor`))

(fn `UserConstructionScript`
  (`parent.UserConstructionScript`))