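; Ghost AI projectile that homes in on a nearby BP_Character tagged "homingTarget" and destroys itself after a short lifetime.
; From BeginPlay, a delay loop repeatedly calls LockOnTarget to refresh the ProjectileMovement homing target, while a second delay handles destruction.
; FindPlayer compares distances to tagged characters against Closest and returns a SceneComponent of the selected HomingTarget.
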(event `LockOnTarget`
  (bind _projectilemovement (`self.ProjectileMovement`))
  (bind _homing_target (`self.FindPlayer`))
  (set `ProjectileMovementComponent.HomingTargetComponent` _homing_target _projectilemovement)
  (set `ProjectileMovementComponent.bIsHomingProjectile` true _projectilemovement))

(event `self.ReceiveBeginPlay`
  (`self.LockOnTarget` :!label _label)
  (`|ExecutionSequence`
    (:`then_0`
      (`KismetSystemLibrary.Delay` 0.2)
      (goto _label))
    (:`then_1`
      (`KismetSystemLibrary.Delay` 1.0)
      (`self.K2_DestroyActor`))))

(fn `FindPlayer`
  (returns (`Homing Target` :type "SceneComponent Object Reference"))
  (bind _outactors (`GameplayStatics.GetAllActorsOfClassWithTag` "/Game/GhostGame/Blueprints/BP_Character.BP_Character_C" "homingTarget"))
  (for _array_element _outactors
    (bind _returnvalue (`KismetMathLibrary.VSize` (- (`self.K2_GetActorLocation` _array_element) (`self.K2_GetActorLocation`))))
    (if (< _returnvalue (`self.Closest`))
      (set `self.Closest` _returnvalue)
      (set `self.HomingTarget` _array_element)))
  (return (`self.GetComponentByClass` (`self.HomingTarget`) "/Script/Engine.SceneComponent")))

(fn `UserConstructionScript`)