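; Sniper projectile that homes in on the closest BP_Character tagged "homingTarget" and damages any BP_Character it hits.
; A looping delay from BeginPlay repeatedly runs FindPlayer and points ProjectileMovement at the first child component of that character's capsule.
; Sphere hits spawn an emitter and destroy the projectile, except against the one BP_BaseGhost cached in IgnoreArray at spawn.
; A lifetime timeout also destroys it.
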(event `LockOnTarget`
  (bind _projectilemovement (`self.ProjectileMovement`))
  ;[1 1 1] Homing on Player
  (bind _homing_target (`self.FindPlayer`))
  (set `ProjectileMovementComponent.HomingTargetComponent` (`SceneComponent.GetChildComponent` (`Character.CapsuleComponent` _homing_target) 0) _projectilemovement)
  (set `ProjectileMovementComponent.bIsHomingProjectile` true _projectilemovement))

(event `self.ReceiveBeginPlay`
  ;[1 1 1] Homing on Player
  (bind _returnvalue (`GameplayStatics.GetActorOfClass` "/Game/GhostGame/AI/GhostNormies/BP_BaseGhost.BP_BaseGhost_C"))
  (`KismetArrayLibrary.Array_Add` (`self.IgnoreArray`) _returnvalue)
  (`self.LockOnTarget` :!label _label)
  (`|ExecutionSequence`
    (:`then_0`
      (`KismetSystemLibrary.Delay` 0.2)
      (goto _label))
    (:`then_1`
      (`KismetSystemLibrary.Delay` 6.0)
      (`self.K2_DestroyActor`))))

(event `self.Sphere1.OnComponentHit`
  (params (HitComponent :type "PrimitiveComponent Object Reference") (OtherActor :type "Actor Object Reference") (OtherComp :type "PrimitiveComponent Object Reference") (NormalImpulse :type "Vector Structure") (Hit :type "HitResult Structure (by ref)"))
  ;[1 1 1] Deal Damage + Delete in Hit
  (bind _asbp_character (cast `/Game/GhostGame/Blueprints/BP_Character` OtherActor)
    (:`then`
      (`/Game/GhostGame/Blueprints/BP_Character.Take Damage` _asbp_character 0.25))
    (:`CastFailed`
      _))
  (`GameplayStatics.SpawnEmitterAttached` null)
  (if (== (`KismetArrayLibrary.Array_Find` (`self.IgnoreArray`) OtherActor) -1)
    (`self.K2_DestroyActor`)))

(fn `FindPlayer`
  (returns (`Homing Target` :type "/Game/GhostGame/Blueprints/BP_Character Object Reference"))
  (bind _outactors (`GameplayStatics.GetAllActorsOfClassWithTag` "/Game/GhostGame/Blueprints/BP_Character.BP_Character_C" "homingTarget"))
  (for _array_element _outactors
    (bind _returnvalue (`KismetMathLibrary.VSize` (- (`self.K2_GetActorLocation` _array_element) (`self.K2_GetActorLocation`))))
    (if (< _returnvalue (`self.Closest`))
      (set `self.Closest` _returnvalue)
      (set `self.HomingTarget` _array_element)))
  (return (`self.HomingTarget`)))

(fn `UserConstructionScript`)