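; BP_BaseGhost is the base enemy ghost, which plays a drone sound and chases the player with a bobbing mesh.
; It re-issues AI MoveTo toward the player's FPS camera on a short delayed loop and bobs via a sine offset each tick.
; Tick also refreshes its health bar and, at zero health, notifies BP_Gamemode, calls an empty pre-cull hook, then self-destroys.
; On destruction it plays a death sound and spawns a health pickup.
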(event `self.ReceiveBeginPlay`
  (`GameplayStatics.PlaySound2D` "/Game/GhostGame/Audio/SC_GhostDrone.SC_GhostDrone" 1.0 1.0 0.0 null null false)
  (`|ExecutionSequence`
    (:`then_0`
      (bind _asbp_character (cast `/Game/GhostGame/Blueprints/BP_Character` (`GameplayStatics.GetPlayerCharacter` 0)))
      (set `self.As BP Character` _asbp_character)
      (`self.FollowPlayer`))
    (:`then_1`
      (`self.UpdateHealthBar`)
      (set `self.Return Value Location Z` (.z (.location (`SceneComponent.GetRelativeTransform` (`self.Mesh`))))))))

(event `self.ReceiveTick`
  (params (DeltaSeconds :type "Float (single-precision)"))
  ;[1 1 1] Bopping up and down
  (`SceneComponent.K2_SetRelativeLocation` (`self.Mesh`) (`KismetMathLibrary.MakeVector` 0.0 0.0 (+ (`self.Return Value Location Z`) (* (`self.BoppingDistance`) (`KismetMathLibrary.DegSin` (* (`self.GetGameTimeSinceCreation`) (`self.BoppingSpeed`)))))) false false)
  (`self.UpdateHealthBar`)
  (`self.CheckHealth`))

(event `FollowPlayer`
  ;[0.05098 0.05098 0.05098] Follow player
  (`|AIMoveTo` self (`SceneComponent.K2_GetComponentLocation` (`/Game/GhostGame/Blueprints/BP_Character.FPS_Camera` (`self.As BP Character`))) null 0.0
    (:`then`
      (`KismetSystemLibrary.Delay` 0.2)
      (`self.FollowPlayer`))))

(event `self.ReceiveDestroyed`
  (bind _returnvalue (`self.GetTransform`))
  (`GameplayStatics.PlaySound2D` "/Game/GhostGame/Audio/SC_GhostDeath.SC_GhostDeath" 1.0 1.0 0.0 null null)
  (`|SpawnActorFromClass` "/Game/GhostGame/Blueprints/BP_HealthPickup.BP_HealthPickup_C" (`KismetMathLibrary.MakeTransform` (`KismetMathLibrary.MakeVector` (.x (.location _returnvalue)) (.y (.location _returnvalue)) 30.0)) "Undefined" "MultiplyWithRoot" null null))

(fn `AdditionalLogicBeforeCull`)

(fn `CheckHealth`
  (if (<= (`self.Health`) 0.0)
    (`KismetSystemLibrary.PrintString` "Ghost Killed")
    (bind _asbp_gamemode (cast `/Game/GhostGame/Blueprints/BP_Gamemode` (`GameplayStatics.GetGameMode`)))
    (`/Game/GhostGame/Blueprints/BP_Gamemode.Ghost Killed` _asbp_gamemode)
    (`|ExecutionSequence`
      (:`then_0`
        (`self.AdditionalLogicBeforeCull`))
      (:`then_1`
        (`self.K2_DestroyActor`)))))

(fn `SetHealth`
  (params (`New Health` :type "Float (double-precision)"))
  (set `self.Health` `New Health`))

(fn `SetMaxHealth`
  (params (NewMaxHealth :type "Float (double-precision)"))
  (set `self.MaxHealth` NewMaxHealth))

(fn `UpdateHealthBar`
  (bind _asbp_health_bar (cast `/Game/GhostGame/AI/BP_HealthBar` (`WidgetComponent.GetUserWidgetObject` (`self.HealthBar`))))
  (set `/Game/GhostGame/AI/BP_HealthBar.Health` (/ (`self.Health`) (`self.MaxHealth`)) _asbp_health_bar)
  (return))

(fn `UserConstructionScript`)