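; BP_Sniper_Ghost is a ghost enemy that turns to face the player and fires projectiles at a steady interval.
; Tick runs a Delay that acts as the fire timer, then, if CanAttack is set, spawns a BP_GhostProjectile and plays the attack animation.
; Each frame it also bobs the mesh on a sine wave around its starting height and snaps the actor's rotation toward BP_Character.
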(event `self.ReceiveBeginPlay`
  (`self.UpdateHealthBar`)
  (set `self.Return Value Location Z` (.z (.location (`SceneComponent.GetRelativeTransform` (`self.Mesh`))))))

(event `self.ReceiveTick`
  (params (DeltaSeconds :type "Float (single-precision)"))
  (bind (_returnvalue_location _returnvalue_rotation) (`KismetMathLibrary.BreakTransform` (`SceneComponent.K2_GetComponentToWorld` (`self.ProjectileSpawn`))))
  (`parent.ReceiveTick` DeltaSeconds)
  (`|ExecutionSequence`
    (:`then_0`
      (`KismetSystemLibrary.Delay` 0.8)
      ;[1 1 1] Fire Projectile
      (`KismetSystemLibrary.PrintString` "FIRE!!")
      (if (`self.CanAttack`)
        (`|SpawnActorFromClass` "/Game/GhostGame/AI/BP_GhostProjectile.BP_GhostProjectile_C" (`KismetMathLibrary.MakeTransform` _returnvalue_location _returnvalue_rotation (0.5 0.5 0.5)) "AlwaysSpawn" "MultiplyWithRoot" null null)
        (`SkeletalMeshComponent.PlayAnimation` (`self.Mesh`) "/Game/LAUREN_ENEMYS/SHOOTER_GHOST/ATTACK/Shooter_Rigged_attack_Anim.Shooter_Rigged_attack_Anim" false)))
    (:`then_1`
      ;[1 1 1] Bopping up and down
      (`SceneComponent.K2_SetRelativeLocation` (`self.Mesh`) (`KismetMathLibrary.MakeVector` 0.0 0.0 (+ (`self.Return Value Location Z`) (* (`self.BoppingDistance`) (`KismetMathLibrary.DegSin` (* (`self.GetGameTimeSinceCreation`) (`self.BoppingSpeed`)))))) false false))
    (:`then_2`
      ;[1 1 1] Rotating to face Player
      (bind _asbp_character (cast `/Game/GhostGame/Blueprints/BP_Character` (`GameplayStatics.GetPlayerCharacter` 0)))
      (`self.K2_SetActorRotation` (`KismetMathLibrary.FindLookAtRotation` (`self.K2_GetActorLocation`) (`self.K2_GetActorLocation` _asbp_character))))))

(fn `UserConstructionScript`
  (`parent.UserConstructionScript`))