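; BP_RangeGhost is a ranged ghost enemy that fires projectiles while CanAttack is true.
; A one-second Delay on Tick paces the attack, which prints a debug string, spawns a half-scale BP_GhostProjectile at ProjectileSpawn and plays the attack animation.
; Tick also sets the player character's rotation, not the ghost's, to the look-at direction from ghost to player.
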(event `self.ReceiveBeginPlay`
  (`parent.ReceiveBeginPlay`))

(event `self.ReceiveTick`
  (params (DeltaSeconds :type "Float (single-precision)"))
  (bind (_returnvalue_location _returnvalue_rotation) (`KismetMathLibrary.BreakTransform` (`SceneComponent.K2_GetComponentToWorld` (`self.ProjectileSpawn`))))
  (`parent.ReceiveTick` DeltaSeconds)
  (`|ExecutionSequence`
    (:`then_0`
      (`KismetSystemLibrary.Delay` 1.0)
      (`KismetSystemLibrary.PrintString` "FIRE!!")
      (if (`self.CanAttack`)
        (`|SpawnActorFromClass` "/Game/GhostGame/AI/BP_GhostProjectile.BP_GhostProjectile_C" (`KismetMathLibrary.MakeTransform` _returnvalue_location _returnvalue_rotation (0.5 0.5 0.5)) "Undefined" "MultiplyWithRoot" null null)
        (`SkeletalMeshComponent.PlayAnimation` (`self.Mesh`) "/Game/LAUREN_ENEMYS/SHOOTER_GHOST/ATTACK/Shooter_Rigged_attack_Anim.Shooter_Rigged_attack_Anim" false)))
    (:`then_1`
      (bind _asbp_character (cast `/Game/GhostGame/Blueprints/BP_Character` (`GameplayStatics.GetPlayerCharacter` 0)))
      (`self.K2_SetActorRotation` _asbp_character (`KismetMathLibrary.FindLookAtRotation` (`self.K2_GetActorLocation`) (`self.K2_GetActorLocation` _asbp_character)) false))))

(fn `UserConstructionScript`
  (`parent.UserConstructionScript`))