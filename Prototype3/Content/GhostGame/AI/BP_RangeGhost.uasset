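; BP_RangeGhost is a ranged ghost enemy that spawns BP_GhostProjectile at its ProjectileSpawn point whenever CanAttack is true.
; A Delay on Tick, after the parent call, paces the logic to roughly half-second intervals, each printing a debug "FIRE!!" before the attack check.
; Each pass also sets the player character's rotation, not the ghost's, to the look-at direction from ghost to player.
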(event `self.ReceiveBeginPlay`
  (`parent.ReceiveBeginPlay`))

(event `self.ReceiveTick`
  (params (DeltaSeconds :type "Float (single-precision)"))
  (`parent.ReceiveTick` DeltaSeconds)
  (`KismetSystemLibrary.Delay` 0.5)
  (`KismetSystemLibrary.PrintString` "FIRE!!")
  (bind _asbp_character (cast `/Game/GhostGame/Blueprints/BP_Character` (`GameplayStatics.GetPlayerCharacter` 0)))
  (`self.K2_SetActorRotation` _asbp_character (`KismetMathLibrary.FindLookAtRotation` (`self.K2_GetActorLocation`) (`self.K2_GetActorLocation` _asbp_character)) false)
  (if (`self.CanAttack`)
    (`|SpawnActorFromClass` "/Game/GhostGame/AI/BP_GhostProjectile.BP_GhostProjectile_C" (`SceneComponent.K2_GetComponentToWorld` (`self.ProjectileSpawn`)) "Undefined" "MultiplyWithRoot" null null)))

(fn `UserConstructionScript`
  (`parent.UserConstructionScript`))