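; Base ghost enemy that chases the player, damages them on contact and reports its death to the game mode.
; A recursive AIMoveTo loop re-targets the player every short delay and holds position when close.
; Tick damages overlapping characters with a timer-reset cooldown, bobs the mesh on a sine wave, updates the health bar widget and checks for death.
; At zero health it notifies BP_Gamemode and destroys itself.
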(event `ResetDamage`
  (set `self.bHasDamaged` false))

(event `self.ReceiveTick`
  (params (DeltaSeconds :type "Float (single-precision)"))
  ;[1 1 1] Bopping up and down
  (`|ExecutionSequence`
    (:`then_0`
      (for _array_element (`PrimitiveComponent.GetOverlappingActors` (`self.DamageBox`) "/Game/GhostGame/Blueprints/BP_Character.BP_Character_C")
        (if (not (`self.bHasDamaged`))
          (bind _asbp_character (cast `/Game/GhostGame/Blueprints/BP_Character` _array_element))
          (`KismetSystemLibrary.PrintString` "Damage Taken")
          (`/Game/GhostGame/Blueprints/BP_Character.TakeDamage` _asbp_character 0.152)
          (`KismetSystemLibrary.K2_SetTimerDelegate` (delegate `ResetDamage`) 1.0)
          (set `self.bHasDamaged` true)
          (break))))
    (:`then_1`
      (`SceneComponent.K2_SetRelativeLocation` (`self.Mesh`) (`KismetMathLibrary.MakeVector` 0.0 0.0 (+ (`self.Return Value Location Z`) (* (`self.BoppingDistance`) (`KismetMathLibrary.DegSin` (* (`self.GetGameTimeSinceCreation`) (`self.BoppingSpeed`)))))) false false)
      (`self.UpdateHealthBar`)
      (`self.CheckHealth`))))

(event `self.ReceiveBeginPlay`
  (`|ExecutionSequence`
    (:`then_0`
      (bind _asbp_character (cast `/Game/GhostGame/Blueprints/BP_Character` (`GameplayStatics.GetPlayerCharacter` 0)))
      (set `self.As BP Character` _asbp_character)
      (`self.FollowPlayer`))
    (:`then_1`
      (`self.UpdateHealthBar`)
      (set `self.Return Value Location Z` (.z (.location (`SceneComponent.GetRelativeTransform` (`self.Mesh`))))))))

(event `FollowPlayer`
  ;[1 1 1] Follow player
  (if (>= (`self.GetDistanceTo` (`self.As BP Character`)) 200.0)
    (`|AIMoveTo` self (0.0 0.0 0.0) (`self.As BP Character`)
      (:`then`
        _))
    (else
      (`|AIMoveTo` self (0.0 0.0 0.0) self
        (:`then`
          _))))
  (`KismetSystemLibrary.Delay` 0.2)
  (`self.FollowPlayer`))

(fn `CheckHealth`
  (if (<= (`self.Health`) 0.0)
    (`KismetSystemLibrary.PrintString` "Ghost Killed")
    (bind _asbp_gamemode (cast `/Game/GhostGame/Blueprints/BP_Gamemode` (`GameplayStatics.GetGameMode`)))
    (`/Game/GhostGame/Blueprints/BP_Gamemode.Ghost Killed` _asbp_gamemode)
    (`self.K2_DestroyActor`)))

(fn `UpdateHealthBar`
  (bind _asbp_health_bar (cast `/Game/GhostGame/AI/BP_HealthBar` (`WidgetComponent.GetUserWidgetObject` (`self.HealthBar`))))
  (set `/Game/GhostGame/AI/BP_HealthBar.Health` (`self.Health`) _asbp_health_bar)
  (return))

(fn `UserConstructionScript`)