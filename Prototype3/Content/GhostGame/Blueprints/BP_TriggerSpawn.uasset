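; Trigger actor that spawns a ghost AI when the player character enters its box.
; On BeginPlay it calls AddGhostToLevel on BP_Gamemode, registering its ghost before any spawn happens.
; The first overlap by an actor whose display name equals "BP_Character" passes a DoOnce and spawns the GhostToSpawn class at the WorldSpawnPoint's location and rotation.
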(event `self.ReceiveBeginPlay`
  (bind _asbp_gamemode (cast `/Game/GhostGame/Blueprints/BP_Gamemode` (`GameplayStatics.GetGameMode`)))
  (`/Game/GhostGame/Blueprints/BP_Gamemode.AddGhostToLevel` _asbp_gamemode))

(event `self.Box.OnComponentBeginOverlap`
  (params (OverlappedComponent :type "PrimitiveComponent Object Reference") (OtherActor :type "Actor Object Reference") (OtherComp :type "PrimitiveComponent Object Reference") (OtherBodyIndex :type Integer) (bFromSweep :type Boolean) (SweepResult :type "HitResult Structure (by ref)"))
  (bind (_returnvalue_location _returnvalue_rotation) (`KismetMathLibrary.BreakTransform` (`SceneComponent.K2_GetComponentToWorld` (`Actor.RootComponent` (`self.WorldSpawnPoint`)))))
  ;[1 1 1] Spawn Ghost
  (if (`KismetStringLibrary.EqualEqual_StrStr` (`KismetSystemLibrary.GetDisplayName` OtherActor) "BP_Character")
    (`/Engine/EditorBlueprintResources/StandardMacros.DoOnce` false
      (:`Completed`
        (`KismetSystemLibrary.PrintString` "Spawning")
        (`AIBlueprintHelperLibrary.SpawnAIFromClass` (`self.GhostToSpawn`) null _returnvalue_location _returnvalue_rotation false null)))))

(fn `UserConstructionScript`)