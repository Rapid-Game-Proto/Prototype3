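; Base ghost spawn point that registers a ghost with the gamemode at BeginPlay.
; Interact shows timed dialogue and spawns the ghost class with Niagara effects, only once.
; A box overlap toggles the prompt text and in-range flag, while Tick yaws the box toward the player and updates a hold-progress widget.
; A BP_TankGhost entering GhostTrigger turns on the mesh's physics and pushes it.
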(event `self.ReceiveBeginPlay`
  (bind _asbp_gamemode (cast `/Game/GhostGame/Blueprints/BP_Gamemode` (`GameplayStatics.GetGameMode`)))
  (`/Game/GhostGame/Blueprints/BP_Gamemode.AddGhostToLevel` _asbp_gamemode))

(event `/Game/GhostGame/Blueprints/BP_Interact.Interact`
  (params (TimeHeld :type "Float (double-precision)"))
  (bind (_returnvalue_location _returnvalue_rotation) (`KismetMathLibrary.BreakTransform` (`SceneComponent.K2_GetComponentToWorld` (`self.SpawnPoint`))))
  ;[1 1 1] Spawn Ghost
  (if (and (`self.PlayerInRange`) (>= TimeHeld 5.0))
    _
    (else
      _))
  (`KismetSystemLibrary.PrintText` (`self.Text`))
  (bind _asbp_character (cast `/Game/GhostGame/Blueprints/BP_Character` (`GameplayStatics.GetPlayerCharacter` 0)))
  (bind _gui_widget (`/Game/GhostGame/Blueprints/BP_Character.GUI Widget` _asbp_character))
  (`/Game/GhostGame/Blueprints/BP_GUI.SetDialogue` _gui_widget (`self.Text`))
  (`|ExecutionSequence`
    (:`then_0`
      (`/Engine/EditorBlueprintResources/StandardMacros.DoOnce` false
        (:`Completed`
          (`AIBlueprintHelperLibrary.SpawnAIFromClass` (`self.GhostToSpawn`) null _returnvalue_location _returnvalue_rotation false null)
          (`NiagaraFunctionLibrary.SpawnSystemAtLocation` "/Game/GhostGame/VFX/GhostAppear_VFX_2.GhostAppear_VFX_2" _returnvalue_location (struct) (3.0 3.0 3.0))
          (`NiagaraFunctionLibrary.SpawnSystemAtLocation` "/Game/GhostGame/VFX/GhostAppear_VFX_1.GhostAppear_VFX_1" _returnvalue_location (struct) (3.0 3.0 3.0)))))
    (:`then_1`
      (`KismetSystemLibrary.Delay` 3.0)
      (`/Game/GhostGame/Blueprints/BP_GUI.SetDialogue` _gui_widget ""))))

(event `self.Box.OnComponentBeginOverlap`
  (params (OverlappedComponent :type "PrimitiveComponent Object Reference") (OtherActor :type "Actor Object Reference") (OtherComp :type "PrimitiveComponent Object Reference") (OtherBodyIndex :type Integer) (bFromSweep :type Boolean) (SweepResult :type "HitResult Structure (by ref)"))
  (cast `/Game/GhostGame/Blueprints/BP_Character` OtherActor)
  (`SceneComponent.SetHiddenInGame` (`self.TextRender`) false false)
  (set `self.PlayerInRange` true))

(event `self.Box.OnComponentEndOverlap`
  (params (OverlappedComponent :type "PrimitiveComponent Object Reference") (OtherActor :type "Actor Object Reference") (OtherComp :type "PrimitiveComponent Object Reference") (OtherBodyIndex :type Integer))
  (cast `/Game/GhostGame/Blueprints/BP_Character` OtherActor)
  (`SceneComponent.SetHiddenInGame` (`self.TextRender`) true false)
  (set `self.PlayerInRange` false))

(event `self.ReceiveTick`
  (params (DeltaSeconds :type "Float (single-precision)"))
  (bind _returnvalue (`GameplayStatics.GetActorOfClass` "/Game/GhostGame/Blueprints/BP_Character.BP_Character_C"))
  (bind (_returnvalue_roll _returnvalue_pitch _returnvalue_yaw) (`KismetMathLibrary.BreakRotator` (`KismetMathLibrary.FindRelativeLookAtRotation` (`self.GetTransform`) (`self.K2_GetActorLocation` _returnvalue))))
  (`SceneComponent.K2_SetRelativeRotation` (`self.Box`) (`KismetMathLibrary.MakeRotator` 0.0 0.0 _returnvalue_yaw) false false)
  (`self.UpdateProgress`))

(event `self.GhostTrigger.OnComponentBeginOverlap`
  (params (OverlappedComponent :type "PrimitiveComponent Object Reference") (OtherActor :type "Actor Object Reference") (OtherComp :type "PrimitiveComponent Object Reference") (OtherBodyIndex :type Integer) (bFromSweep :type Boolean) (SweepResult :type "HitResult Structure (by ref)"))
  (bind _objectmesh (`self.ObjectMesh`))
  (cast `/Game/GhostGame/AI/BP_TankGhost` OtherActor)
  (`PrimitiveComponent.SetSimulatePhysics` _objectmesh true)
  (`PrimitiveComponent.AddForce` _objectmesh (0.0 1500.0 0.0) "None" false))

(fn `UpdateProgress`
  (bind _aswbp_progress_bar (cast `/Game/GhostGame/Blueprints/WBP_ProgressBar` (`WidgetComponent.GetUserWidgetObject` (`self.ProgressMeter`))))
  (set `/Game/GhostGame/Blueprints/WBP_ProgressBar.Progress` (- 1.0 (/ (`self.InteractTime`) 5.0)) _aswbp_progress_bar)
  (return))

(fn `UserConstructionScript`)