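; BP_PopcornChair is a ghost-game actor that rises into the air when its Lift event is called.
; Lift stores the root component's current world location and a target 400 units above it, then plays a timeline from the start.
; Each timeline update lerps the root between those points using the LiftPercentage track, without sweep.
; BeginPlay, overlap and Tick are unused.
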(event `Lift`
  (bind _output_get (set `self.StartPos` (`SceneComponent.K2_GetComponentLocation` (`self.DefaultSceneRoot`))))
  (set `self.EndPos` (+ _output_get (0.0 0.0 400.0)))
  (bind (_direction _liftpercentage) (`Timeline|Timeline` :!via `PlayFromStart`)
    (:`Update`
      (`SceneComponent.K2_SetWorldLocation` (`self.DefaultSceneRoot`) (`KismetMathLibrary.VLerp` (`self.StartPos`) (`self.EndPos`) _liftpercentage) false false))))

(fn `UserConstructionScript`)