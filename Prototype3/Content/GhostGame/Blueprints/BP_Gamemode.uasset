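; Game mode for the ghost game, handling level progression, player death, money, pausing, valuables and achievement popups.
; It counts ghosts in the level and activates the door when none remain, then resets on advancing to the next level.
; Valuable pickups are flagged per level, and collecting the first three triggers an achievement.
; Achievement widgets slide up and fade out through two chained timelines before being removed.
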(event `ControlAchievement`
  (bind _achievementwidget (`self.AchievementWidget`))
  (`UserWidget.SetPositionInViewport` _achievementwidget (660.0 600.0) true)
  (bind (_direction _achievementpopuplerp) (`Timeline|AchievementPopUp` :!via `PlayFromStart`)
    (:`Update`
      (`UserWidget.SetPositionInViewport` _achievementwidget (`KismetMathLibrary.MakeVector2D` 660.0 (`KismetMathLibrary.Lerp` 600.0 565.0 _achievementpopuplerp)) true))
    (:`Finished`
      (`KismetSystemLibrary.Delay` 2.0)
      (bind (_direction_2 _fadeoutlerp) (`Timeline|DisapearAchievement` :!via `PlayFromStart`)
        (:`Update`
          (`Widget.SetRenderOpacity` _achievementwidget (- 1.0 _fadeoutlerp)))
        (:`Finished`
          (`Widget.RemoveFromParent` _achievementwidget))))))

(event `GoToLevelSelect`
  (`KismetSystemLibrary.Delay` 3.0)
  (`GameplayStatics.OpenLevel` "LevelSelectMenu")
  (set `PlayerController.bShowMouseCursor` false (`GameplayStatics.GetPlayerController` 0))
  (`WidgetLayoutLibrary.RemoveAllWidgets`))

(fn `AddGhostToLevel`
  (set `self.GhostsInLevel` (+ (`self.GhostsInLevel`) 1)))

(fn `CheckValuableItems`
  (bind _levelvaluablecollection (`self.LevelValuableCollection`))
  (if (`self.ValuableAchievementGet?`)
    _
    (elif (and (and (`|GetArrayItem` _levelvaluablecollection) (`|GetArrayItem` _levelvaluablecollection 1)) (`|GetArrayItem` _levelvaluablecollection 2))
      (`self.ShowAchievement` 5))))

(fn `CollectValuable`
  (params (`Level Num` :type Integer))
  (`KismetArrayLibrary.Array_Set` (`self.LevelValuableCollection`) `Level Num` true)
  (`KismetSystemLibrary.PrintString` (`KismetTextLibrary.Conv_TextToString` (`|FormatText` "Picked up Valuable from Level {LevelNum}" `Level Num`)))
  (`self.CheckValuableItems`))

(fn `Ghost Killed`
  (bind _output_get (set `self.GhostsInLevel` (- (`self.GhostsInLevel`) 1)))
  (if (<= _output_get 0)
    (set `self.bDoorActive` true)))

(fn `LevelOver`
  (params (Money :type "Float (double-precision)"))
  (set `self.PlayerMoney` (+ (`self.PlayerMoney`) Money))
  (cast `/Game/GhostGame/Blueprints/BP_Character` (`GameplayStatics.GetPlayerCharacter` 0)))

(fn `Next Level`
  (set `self.bDoorActive` false)
  (set `self.GhostsInLevel` 0)
  (`GameplayStatics.OpenLevelBySoftObjectPtr` "/Game/BaseContent/FirstPerson/Maps/FirstPersonMap.FirstPersonMap")
  (set `self.levelID` (+ (`self.levelID`) 1)))

(fn `PauseGame`
  (bind _returnvalue (`GameplayStatics.IsGamePaused`))
  (`GameplayStatics.SetGamePaused` (not _returnvalue))
  (set `PlayerController.bShowMouseCursor` _returnvalue (`GameplayStatics.GetPlayerController` 0)))

(fn `PlayerDeath`
  (`WidgetLayoutLibrary.RemoveAllWidgets`)
  (bind _returnvalue (`|CreateWidget` "/Game/GhostGame/Maps+HUD/WBP_Fainted.WBP_Fainted_C"))
  (`UserWidget.AddToViewport` _returnvalue 0)
  (`GameplayStatics.OpenLevel` "MainMenu")
  (set `PlayerController.bShowMouseCursor` false (`GameplayStatics.GetPlayerController` 0))
  (`WidgetLayoutLibrary.RemoveAllWidgets`))

(fn `ShowAchievement`
  (params (AchievementIndex :type Integer))
  (`KismetSystemLibrary.PrintString` "ACHIEVMENT GOING THORUGH")
  (bind _returnvalue (`|CreateWidget` "/Game/GhostGame/Maps+HUD/WBP_Achievements.WBP_Achievements_C" (`GameplayStatics.GetPlayerController` 0)))
  (set `/Game/GhostGame/Maps+HUD/WBP_Achievements.DisplayedAchievement` AchievementIndex _returnvalue)
  (bind _output_get (set `self.AchievementWidget` _returnvalue))
  (`UserWidget.AddToViewport` _output_get 0)
  (`self.ControlAchievement`))

(fn `UserConstructionScript`)