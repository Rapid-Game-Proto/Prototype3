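; Cinema staff double door interactable that swings both leaves open when its inherited object action fires.
; A dot product between the Direction component's forward vector and the offset from BP_Character determines which side the player is on, setting the swing direction.
; Each leaf gets a quarter-turn target with a randomized offset, and one timeline lerps both world rotations toward their targets.
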(event `self.ReceiveTick`
  (params (DeltaSeconds :type "Float (single-precision)"))
  (`parent.ReceiveTick` DeltaSeconds))

(event `self.DoActionOfObject`
  (`parent.DoActionOfObject`)
  (bind _output_get (set `self.StartRotationRightDoor` (`SceneComponent.K2_GetComponentRotation` (`self.StaticMesh`))))
  (`self.Get Player Orientation`
    (:`Infront`
      (bind _returnvalue (+ (.yaw _output_get) (`KismetMathLibrary.RandomFloatInRange` -10.0 -20.0)))
      (set `self.EndRotationRightDoor` (`KismetMathLibrary.MakeRotator` (.roll _output_get) (.pitch _output_get) (+ _returnvalue 90.0))))
    (:`Behind`
      (set `self.EndRotationRightDoor` (`KismetMathLibrary.MakeRotator` (.roll _output_get) (.pitch _output_get) (+ _returnvalue -90.0)))))
  (bind _output_get_2 (set `self.StartRotationLeftDoor` (`SceneComponent.K2_GetComponentRotation` (`self.LeftDoor`))))
  (`self.Get Player Orientation`
    (:`Infront`
      (bind _returnvalue_2 (+ (.yaw _output_get_2) (`KismetMathLibrary.RandomFloatInRange` 10.0 20.0)))
      (set `self.EndRotationLeftDoor` (`KismetMathLibrary.MakeRotator` (.roll _output_get_2) (.pitch _output_get_2) (+ _returnvalue_2 -90.0)))
      (bind (_direction _dooropentrack) (`Timeline|Timeline` :!via `PlayFromStart` :!label _label)
        (:`Update`
          (`SceneComponent.K2_SetWorldRotation` (`self.StaticMesh`) (`KismetMathLibrary.RLerp` (`self.StartRotationRightDoor`) (`self.EndRotationRightDoor`) _dooropentrack) false false)
          (`SceneComponent.K2_SetWorldRotation` (`self.LeftDoor`) (`KismetMathLibrary.RLerp` (`self.StartRotationLeftDoor`) (`self.EndRotationLeftDoor`) _dooropentrack) false false))))
    (:`Behind`
      (set `self.EndRotationLeftDoor` (`KismetMathLibrary.MakeRotator` (.roll _output_get_2) (.pitch _output_get_2) (+ _returnvalue_2 90.0)))
      (goto _label :!via `PlayFromStart`))))

(fn `UserConstructionScript`
  (`parent.UserConstructionScript`))